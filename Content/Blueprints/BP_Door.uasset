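; Sliding door actor that lowers its mesh to open and raises it to close, opening automatically on BeginPlay.
; Open and Close events, guarded by an IsOpen flag, play or reverse one Timeline that lerps the mesh's relative location.
; Each also switches four spotlights and an indicator mesh material between green for open and red for closed.
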(event `self.ReceiveBeginPlay`
  (`self.open`))

(event `open`
  (if (not (`self.IsOpen`))
    (set `self.IsOpen` true)
    (`LightComponent.SetLightColor` (`self.SpotLight`) (struct :`R` 0.787975 :`G` 0.854167 :`B` 0.496821 :`A` 1.0) true)
    (`LightComponent.SetLightColor` (`self.SpotLight1`) (struct :`R` 0.787975 :`G` 0.854167 :`B` 0.496821 :`A` 1.0) true)
    (`LightComponent.SetLightColor` (`self.SpotLight2`) (struct :`R` 0.787975 :`G` 0.854167 :`B` 0.496821 :`A` 1.0) true)
    (`LightComponent.SetLightColor` (`self.SpotLight3`) (struct :`R` 0.787975 :`G` 0.854167 :`B` 0.496821 :`A` 1.0) true)
    (`PrimitiveComponent.SetMaterial` (`self.StaticMesh2`) 0 "/Game/Materials/M_GreenLight.M_GreenLight")
    (bind (_direction _newtrack_0) (`Timeline|Timeline_0` :!label _label)
      (:`Update`
        (`SceneComponent.K2_SetRelativeLocation` (`self.StaticMesh`) (`KismetMathLibrary.VLerp` (0.0 0.0 0.0) (0.0 0.0 -200.0) _newtrack_0) false false)))))

(event `Close`
  (if (`self.IsOpen`)
    (set `self.IsOpen` false)
    (`LightComponent.SetLightColor` (`self.SpotLight1`) (struct :`R` 0.854167 :`G` 0.023079 :`A` 1.0) true)
    (`LightComponent.SetLightColor` (`self.SpotLight`) (struct :`R` 0.854167 :`G` 0.023079 :`A` 1.0) true)
    (`LightComponent.SetLightColor` (`self.SpotLight2`) (struct :`R` 0.854167 :`G` 0.023079 :`A` 1.0) true)
    (`LightComponent.SetLightColor` (`self.SpotLight3`) (struct :`R` 0.854167 :`G` 0.023079 :`A` 1.0) true)
    (`PrimitiveComponent.SetMaterial` (`self.StaticMesh2`) 0 "/Game/Materials/M_RedLight.M_RedLight")
    (goto _label :!via `Reverse`)))

(fn `UserConstructionScript`)